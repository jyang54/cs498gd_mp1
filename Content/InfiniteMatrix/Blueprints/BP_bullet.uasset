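; Projectile actor that destroys enemies and awards points to the actor that fired it.
; The construction script applies the configurable speed to the projectile movement component and sets a short lifespan.
; Box overlaps ignore the player, destroy the bullet on tunnel contact, and on enemy contact destroy the enemy and increment the Shooter's score.
; The bullet itself is not destroyed when it hits an enemy.
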(event OnComponentBeginOverlap(Box)
  (params (OverlappedComponent :type Primitive%20Component%20Object%20Reference) (OtherActor :type Actor%20Object%20Reference) (OtherComp :type Primitive%20Component%20Object%20Reference) (OtherBodyIndex :type Integer) (bFromSweep :type Boolean) (SweepResult :type Hit%20Result%20Structure%20%28by%20ref%29))
  (bind _shooter (Variables|Default|GetShooter))
  (Utilities|Casting|CastToBP_Player OtherActor
    (:CastFailed
      (Utilities|Casting|CastToBP_Tunnel OtherActor
        (:then
          (Actor|DestroyActor))
        (:CastFailed
          (bind _asenemy (Utilities|Casting|CastToEnemy OtherActor))
          (Actor|DestroyActor _asenemy)
          (Development|PrintString "Enemy destroyed")
          (Variables|/Game/InfiniteMatrix/Blueprints/BP_Player.BP_Player_C|SetScore _shooter (+ (Variables|/Game/InfiniteMatrix/Blueprints/BP_Player.BP_Player_C|GetScore _shooter) 1)))))))

(event EventBeginPlay)

(event Collision|EventActorBeginOverlap
  (params (OtherActor :type Actor%20Object%20Reference)))

(event EventTick
  (params (DeltaSeconds :type Float%20%28single-precision%29)))

(fn ConstructionScript
  (Variables|/Script/Engine.ProjectileMovementComponent|SetInitialSpeed (Variables|Default|GetProjectileMovement) (Variables|Default|GetProjectileSpeed))
  (Actor|SetLifeSpan 3.0))